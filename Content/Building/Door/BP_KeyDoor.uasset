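; BP_KeyDoor is a door that opens only for a player holding the key that matches its KeyChannel.
; On interaction it checks the player's keys, prints the locked or unlocked result, and calls Open or Close.
; Open plays a timeline that drives the door's relative yaw, while Close reverses it, and both update the IsDoorOpen flag.
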(event `/Game/GameMode/InteractableInterface.OnInteraction`
  (params (Player :type "/Game/ThirdPersonBP/Blueprints/ThirdPersonCharacter Object Reference"))
  (`/Engine/EditorBlueprintResources/StandardMacros.IsValid` Player
    (:`Is Valid`
      (if (`/Game/ThirdPersonBP/Blueprints/ThirdPersonCharacter.HasKey?` Player (`self.KeyChannel`))
        (`KismetSystemLibrary.PrintString` "Unlocked")
        (`self.Open`)
        (else
          (`KismetSystemLibrary.PrintString` "Locked")
          (`self.Close`))))))

(event `Open`
  (set `self.IsDoorOpen` true)
  (bind (_direction _newtrack_0) (`Timeline|RotationDoorTimeline` :!label _label)
    (:`Update`
      (`SceneComponent.K2_SetRelativeRotation` (`self.Door`) (`KismetMathLibrary.MakeRotator` 0.0 0.0 _newtrack_0) false false))))

(event `Close`
  (set `self.IsDoorOpen` false)
  (goto _label :!via `Reverse`))

(fn `UserConstructionScript`)